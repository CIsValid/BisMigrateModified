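; Vagrancy game state that replaces destroyed ships and asteroids to keep the space around the sun populated.
; On a kill notice, it spawns an enemy ship for PO or a resource ship for CIV, re-rolling the position until it passes a minimum distance from the sun.
; Positions derive from player location, a random vector and sun location.
; Destroyed asteroids respawn with their path and material type passed on.
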(event EventBeginPlay
  (bind _returnvalue (Actor|GetActorOfClass "/Game/Planets/Sun/BP_Sun.BP_Sun_C"))
  (Variables|Default|SetSunRef _returnvalue))

(event EventAsteroidDestroyed
  (params (Path :type Path%20Object%20Reference) (TypeOfMat :type TypesOfResources%20Enum :default "NewEnumerator0"))
  (bind _returnvalue (Game|SpawnActorfromClass "/Game/VFX/VFX/BIS/AsteroidBP.AsteroidBP_C" (Math|Transform|MakeTransform "0, 0, 0" "0, 0, 0" "6.128818,6.128818,6.128818") "AdjustIfPossibleButAlwaysSpawn" 0 0))
  (Variables|/Game/VFX/VFX/BIS/AsteroidBP.AsteroidBP_C|SetpathRef _returnvalue Path)
  (Variables|/Game/VFX/VFX/BIS/AsteroidBP.AsteroidBP_C|SetE%20Type%20Of%20Mat _returnvalue TypeOfMat))

(event EventEnemyKilledNotif
  (params (EnemyType :type EnemyType%20Enum :default "NewEnumerator0") (KillLocation :type Vector :default "0, 0, 0"))
  (bind _returnvalue (Math|Random|RandomRotator true))
  (switch Utilities|FlowControl|Switch|SwitchonEnemyType EnemyType
    (:NewEnumerator0
      (bind (_returnvalue_2 _newpos) (CallFunction|GetRandomPosAroundSun :!label _label))
      (if (> _returnvalue_2 2e+04)
        (Game|SpawnActorfromClass "/Game/AIBehaviour/EnemyBoat/EshipAI.EshipAI_C" (Math|Transform|MakeTransform _newpos _returnvalue "1.000000,1.000000,1.000000") "AdjustIfPossibleButAlwaysSpawn" 0 0)
        (else
          (goto _label))))
    (:NewEnumerator1
      (bind (_returnvalue_3 _newpos_2) (CallFunction|GetRandomPosAroundSun :!label _label_2))
      (if (> _returnvalue_3 2e+04)
        (Game|SpawnActorfromClass "/Game/AIBehaviour/ResourceShip/ResourceShipAI.ResourceShipAI_C" (Math|Transform|MakeTransform _newpos_2 _returnvalue "1.000000,1.000000,1.000000") "AdjustIfPossibleButAlwaysSpawn" 0 0)
        (else
          (goto _label_2))))))

(fn ConstructionScript)

(fn GetRandomPosAroundSun
  (bind _returnvalue (Game|Player|GetPlayerPawn 0))
  (bind _returnvalue_2 (Math|Random|RandomUnitVector))
  (bind _sunref (Variables|Default|GetSunRef))
  (bind _returnvalue_3 (Transformation|GetActorLocation _sunref))
  (bind _returnvalue_4 (Transformation|GetActorLocation _returnvalue))
  (bind _returnvalue_5 (* _returnvalue_4 _returnvalue_2))
  (bind _returnvalue_6 (Math|Vector|Normalize _returnvalue_5))
  (bind _returnvalue_7 (* _returnvalue_6 _returnvalue_3))
  (bind _returnvalue_8 (* _returnvalue_7 2.0))
  (return (Math|Vector|Distance(Vector) _returnvalue_8 _returnvalue_3) _returnvalue_8))