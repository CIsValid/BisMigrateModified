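; Multiplayer player controller that creates the client HUD and in-game menu and handles respawning.
; Escape toggles the menu, switching input mode and cursor, driving menu audio and disabling Boat modes on open.
; UnPossess binds to pawn destruction to notify the game mode; the respawn event spawns a CustomCamera and possesses it after a frame's delay.
; A flip-flop event toggles a radial tool widget and camera lock, with no active caller here.
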(event Custom|ClientDrawHUD
  ;[0 0 0] HUD
  (|CreateInGameHudOverlay))

(event Custom|Server_Respawn
  ;[0 0 0] Respawn
  (|CalledFromServer-RespawnPlayer))

(event Custom|ClientDrawInGameMenu
  (bind _returnvalue (UserInterface|CreateWidget "/Game/Widgets/HUD/InGameMenu.InGameMenu_C"))
  (bind _output_get (Variables|Default|SetInGameMenu _returnvalue))
  (UserInterface|Viewport|AddtoViewport _output_get 0)
  (Widget|SetVisibility (Variables|Default|GetInGameMenu) "Collapsed"))

(event Custom|CheckIfSoundValid
  (params (Sound :type Audio%20Component%20Object%20Reference) (Name :type Name))
  (Utilities|IsValid (Variables|/Script/Engine.AudioComponent|GetSound Sound)
    (:Is%20Valid
      (switch Utilities|FlowControl|Switch|SwitchonEAudioComponentPlayState (Audio|Components|Audio|GetPlayState Sound)
        (:Playing
          _)
        (:Stopped
          (Audio|Components|Audio|Play Sound 0.0 :!label _label))
        (:Paused
          (goto _label))
        (:FadingIn
          _)
        (:FadingOut
          _))
      (Class|AudioParameterControllerInterface|SetTriggerParameter Sound Name))))

(event EventCreateinGameMenu
  (CallFunction|ClientDrawinGameMenu))

(event EventOpenMenu
  (bind _ingamemenu (Variables|Default|GetInGameMenu))
  (if (Variables|Default|GetbIsInMenu)
    (Default|ResetWiget (Variables|Default|GetInGameMenu))
    (Widget|SetVisibility _ingamemenu "Collapsed")
    (Input|SetInputModeGameOnly self)
    (Variables|Default|SetbShowMouseCursor false)
    (Variables|Default|SetbIsInMenu false)
    (CallFunction|CheckifSoundValid (Variables|Default|GetInGameWidgetLoop) "CloseMenu")
    (else
      (Widget|SetVisibility _ingamemenu "Visible")
      (Input|SetInputModeGameandUI self (Variables|Default|GetInGameMenu) "LockOnCapture" false)
      (AI|Navigation|StopMovement self)
      (Variables|Default|SetbShowMouseCursor true)
      (Variables|Default|SetbIsInMenu true)
      (CallFunction|CheckifSoundValid (Variables|Default|GetInGameWidgetLoop) "LoopStart")
      (bind _returnvalue (Actor|GetActorOfClass "/Game/Boat/boat.boat_C"))
      (Default|DisableModes _returnvalue))))

(event EventUnPossess
  (params (UnpossessedPawn :type Pawn%20Object%20Reference))
  ;[0 0 0] Respawn
  (|WhenDeadAskServerToRespawn UnpossessedPawn))

(event EventBeginPlay
  (Input|SetInputModeGameOnly self)
  (Variables|Default|SetbShowMouseCursor false)
  (bind _ascustom_camera (Utilities|Casting|CastToCustomCamera (Pawn|GetControlledPawn)))
  (Variables|Default|SetCharacterRef _ascustom_camera))

(event EventRadialSelectionMenu
  (bind _testhudref (Variables|Default|GetTestHUDRef))
  (bind _radicaltoolwg (Variables|/Game/Widgets/HUD/TestWidget.TestWidget_C|GetRadicalToolWG _testhudref))
  (Utilities|FlowControl|FlipFlop
    (:A
      (Widget|SetVisibility _radicaltoolwg "Visible")
      (Input|SetIgnoreLookInput true)
      (Variables|/Game/Character/CustomCamera.CustomCamera_C|SetbLockCameraMovement (Variables|Default|GetCharacterRef) true)
      (Class|PlayerController|SetMouseLocation self (Variables|/Game/Character/Widgets/RadicalToolWG.RadicalToolWG_C|GetScreen%20Middle%20X _radicaltoolwg) (Variables|/Game/Character/Widgets/RadicalToolWG.RadicalToolWG_C|GetScreen%20Middle%20Y _radicaltoolwg)))
    (:B
      (Widget|SetVisibility _radicaltoolwg "Collapsed")
      (Variables|/Game/Character/CustomCamera.CustomCamera_C|SetbLockCameraMovement (Variables|Default|GetCharacterRef) false)
      (Input|SetInputModeGameOnly self)
      (Class|Controller|ResetIgnoreInputFlags))))

(event EventHoveredMenu
  (CallFunction|CheckifSoundValid (Variables|Default|GetWidgetInteractionComponent) "Hover"))

(event EventPressedMenu
  (CallFunction|CheckifSoundValid (Variables|Default|GetWidgetInteractionComponent) "Press"))

(event EventCreateHUD
  ;[0 0 0] HUD
  (CallFunction|ClientDrawHUD))

(event EventClickedBackMenu
  (CallFunction|CheckifSoundValid (Variables|Default|GetWidgetInteractionComponent) "Back"))

(event Input|KeyboardEvents|Escape
  (params (Key :type Key%20Structure :default "None"))
  (:Pressed
    (CallFunction|OpenMenu)))

(event Input|KeyboardEvents|E
  (params (Key :type Key%20Structure :default "None"))
  ;[1 1 1] Has to change?
)

(event Input|KeyboardEvents|9
  (params (Key :type Key%20Structure :default "None"))
  ;[1 1 1] For debugging
  (:Pressed
    (CallFunction|OpenMenu)))

(fn ConstructionScript)

(event Custom|PlayerIsDead
  (params (DestroyedActor :type Actor%20Object%20Reference))
  (Class|INTGameMode|RespawnPlayer(Message) (Game|GetGameMode) self))