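; Side cannon battery for the boat: aims with the boat's spring arm and fires a broadside from 24 cannon positions.
; While prediction is active, Tick matches the attach point's pitch and yaw to the camera boom, and a looping timer drives the spline trajectory preview.
; Firing shuffles the cannons and spawns projectiles with muzzle particles through a delayed loop, staggering shots after one sound.
; Upgradeable damage passes to each projectile; fire rate is only stored.
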(event Custom|FireCannons
  (params (Cannon :type Scene%20Component%20Object%20Reference))
  (bind _returnvalue (Transformation|GetWorldLocation Cannon))
  (bind _cannonattachpoint (Variables|Default|GetCannonAttachPoint))
  (bind _returnvalue_2 (Math|Vector|GetForwardVector _cannonattachpoint))
  (bind _returnvalue_3 (* _returnvalue_2 1e+03))
  (bind _returnvalue_4 (+ _returnvalue_3 _returnvalue))
  (Utilities|FlowControl|DoOnce false
    (:Completed
      (bind _returnvalue_5 (Game|SpawnActorfromClass "/Game/Boat/BoatProjectiles/CannonTypeProjectile.CannonTypeProjectile_C" (Math|Transform|MakeTransform _returnvalue_4 "0, 0, 0" "1,1,1") "Undefined" 0 0))
      (Variables|/Script/Engine.MovementComponent|SetVelocity (Variables|/Game/Boat/BoatProjectiles/CannonTypeProjectile.CannonTypeProjectile_C|GetProjectileMovement _returnvalue_5) (* _returnvalue_2 1.2e+04))
      (Variables|/Game/Boat/BoatProjectiles/CannonTypeProjectile.CannonTypeProjectile_C|SetDamage _returnvalue_5 (Variables|Default|Getdamage))
      (AddComponent|AddParticleSystemComponent true (Math|Transform|MakeTransform _returnvalue_4 "0, 0, 0" "15.000000,15.000000,15.000000")))))

(event Custom|ReadyCannon
  (bind _cannonattachpoint (Variables|Default|GetCannonAttachPoint))
  (bind _returnvalue (Math|Vector|GetForwardVector _cannonattachpoint))
  (Utilities|Array|Shuffle (Variables|Default|GetCannonArray))
  (Audio|PlaySoundatLocation "/Game/SFX/CannonFire.CannonFire" (Transformation|GetWorldLocation (Variables|Default|GetPredictionPoint)) "0, 0, 0" 1.0 1.0 0.0 0 0 0)
  (bind _arrayelement (Utilities|ForEachLoopwithDelay (Variables|Default|GetCannonArray) (Math|Random|RandomFloatinRange 0.01 0.06))
    (:LoopBody
      (CallFunction|FireCannons _arrayelement)
      (Utilities|FlowControl|DoOnce false) ; enters at Reset
    )
    (:Completed
      (Development|PrintString "Cannons Fired"))))

(event Custom|UpdateUpgradedCannonVars
  (params (damage :type Float%20%28single-precision%29) (fireRate :type Float%20%28single-precision%29))
  (Variables|Default|Setdamage damage)
  (Variables|Default|SetfireRate fireRate))

(event Custom|CreateProjectilePrediction
  (CallFunction|CreateProjectilePath (Transformation|GetWorldLocation (Variables|Default|GetPredictionPoint)) (Math|Vector|GetForwardVector (Variables|Default|GetCannonAttachPoint)) 1.2e+04 42.0 "ECC_WorldStatic" 6.0 1.5 0.0 (Variables|Default|GetSplinePrediction) true "ForOneFrame" (Utilities|Array|MakeArray self (Variables|Default|GetboatRef))))

(event Custom|ReadyPrediction
  (Rendering|SetVisibility (Variables|Default|GetSplineLocation) true true)
  (bind _returnvalue (Utilities|Time|SetTimerbyEvent (EventDispatchers|CreateEvent :!event Custom|CreateProjectilePrediction) 0.1 true))
  (bind _output_get (Variables|Default|SetPredict%20Path%20Event _returnvalue))
  (Variables|Default|SetbGotPredictionLine true))

(event Custom|RemovePredictionLine
  (if (Utilities|Time|IsValidTimerHandle (stale Custom|ReadyPrediction _output_get))
    (Utilities|Time|ClearandInvalidateTimerbyHandle (stale Custom|ReadyPrediction _output_get)))
  (Rendering|SetVisibility (Variables|Default|GetSplineLocation) false true)
  (Variables|Default|SetbGotPredictionLine false))

(event EventTick
  (params (DeltaSeconds :type Float%20%28single-precision%29))
  (bind _boatref (Variables|Default|GetboatRef))
  (bind _cannonattachpoint (Variables|Default|GetCannonAttachPoint))
  (bind _cannonattachpoint_2 (Variables|Default|GetCannonAttachPoint))
  (bind _relativerotation (Variables|/Script/Engine.SceneComponent|GetRelativeRotation _cannonattachpoint))
  (bind _relativerotation_2 (Variables|/Script/Engine.SceneComponent|GetRelativeRotation _cannonattachpoint_2))
  (bind _springarm (Variables|/Game/Boat/boat.boat_C|GetSpringArm _boatref))
  (bind _relativerotation_3 (Variables|/Script/Engine.SceneComponent|GetRelativeRotation _springarm))
  (if (Variables|Default|GetbGotPredictionLine)
    (Transformation|SetRelativeRotation _cannonattachpoint_2 (Math|Rotator|MakeRotator (.roll _relativerotation) (.pitch _relativerotation_3) (.yaw _relativerotation)) false false)
    (Transformation|SetRelativeRotation (Variables|Default|GetCannonAttachPoint) (Math|Rotator|MakeRotator (.roll _relativerotation_2) (.pitch _relativerotation_2) (Class|KismetMathLibrary|ClampAxis (.yaw _relativerotation_3))) false false)))

(event EventBeginPlay
  (Variables|Default|SetCannonArray (Utilities|Array|MakeArray (Variables|Default|GetCannonPos13) (Variables|Default|GetCannonPos2) (Variables|Default|GetCannonPos3) (Variables|Default|GetCannonPos4) (Variables|Default|GetCannonPos5) (Variables|Default|GetCannonPos6) (Variables|Default|GetCannonPos7) (Variables|Default|GetCannonPos8) (Variables|Default|GetCannonPos9) (Variables|Default|GetCannonPos10) (Variables|Default|GetCannonPos11) (Variables|Default|GetCannonPos12) (Variables|Default|GetCannonPos1) (Variables|Default|GetCannonPos14) (Variables|Default|GetCannonPos15) (Variables|Default|GetCannonPos16) (Variables|Default|GetCannonPos17) (Variables|Default|GetCannonPos18) (Variables|Default|GetCannonPos19) (Variables|Default|GetCannonPos20) (Variables|Default|GetCannonPos21) (Variables|Default|GetCannonPos22) (Variables|Default|GetCannonPos23) (Variables|Default|GetCannonPos24)))
  (bind _asboat (Utilities|Casting|CastToboat (Actor|GetParentActor)))
  (Variables|Default|SetboatRef _asboat)
  ;[0.0152 0.6218 1] UPGRADE CANNON VARS
  (CallFunction|UpdateUpgradedCannonVars 1.0 5.0))

(fn ConstructionScript
  (|CallParentFunction))