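; Boat sails Blueprint that fades three sail stages in and out as the parent boat's thrust level changes.
; Looping timers, used in place of Tick, drive updates from the thrust level read off the boat.
; A switch on that level uses DoOnce gates to fire each transition once per change.
; Per-stage timelines animate material Opacity forward or in reverse, with stage 2 and 3 alphas tracked for step-down to level 1.
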(event Custom|ChangeSails
  ;[0 0 0] Use boat reference to fetch the Thruster Speed and make a veriable in our animation blueprint
  (Variables|Default|SetSailThruster (Utilities|Enum|ByteToEnumBoatThrustSpeed (Variables|/Game/Boat/boat.boat_C|GetThrustLevel (Variables|Default|GetAs%20Boat)))))

(event Custom|ChangeShaderParamSail3
  (params (ObjectWithMat :type Mesh%20Component%20Object%20Reference) (ParameterName :type Name))
  ;[0.1198 0.2804 0.5052] Sail Timelines for transition
  (bind _alpha (Timeline|ChangeShaderTimelineSail3 Play)
    (:Update
      (Rendering|Material|SetScalarParameterValueonMaterials ObjectWithMat ParameterName _alpha)
      (Variables|Default|SetThurster3Alpha _alpha))))

(event Custom|RevertShaderChangeSail3
  (params (ObjectWithMat :type Mesh%20Component%20Object%20Reference))
  ;[0.1198 0.2804 0.5052] Sail Timelines for transition
  (bind _alpha (Timeline|ChangeShaderTimelineSail3 Reverse)
    (:Update
      (Rendering|Material|SetScalarParameterValueonMaterials (stale Custom|ChangeShaderParamSail3 ObjectWithMat) (stale Custom|ChangeShaderParamSail3 ParameterName) _alpha)
      (Variables|Default|SetThurster3Alpha _alpha))))

(event Custom|ChangeSailShaderCallable
  (bind _sails_stage1 (Variables|Default|GetSails_Stage1))
  (switch Utilities|FlowControl|Switch|SwitchonBoatThrustSpeed (Variables|Default|GetSailThruster)
    (:NewEnumerator0
      (Utilities|FlowControl|Sequence
        (:then_0
          (Utilities|FlowControl|DoOnce true :!label _label
            (:Completed
              (CallFunction|RevertShaderChange _sails_stage1)
              (CallFunction|RevertShaderChangeSail2 (Variables|Default|GetSails_Stage2))
              (CallFunction|RevertShaderChangeSail3 (Variables|Default|GetSails_Stage3)))))
        (:then_1
          (goto _label_2 Reset))
        (:then_2
          (goto _label_3 Reset))
        (:then_3
          (goto _label_4 Reset))))
    (:NewEnumerator1
      (Utilities|FlowControl|Sequence
        (:then_0
          (Utilities|FlowControl|DoOnce false :!label _label_2
            (:Completed
              (CallFunction|ChangeShaderParam _sails_stage1 "Opacity")
              (Utilities|FlowControl|Sequence
                (:then_0
                  (if (> (Variables|Default|GetThurster2Alpha) 0.0)
                    (CallFunction|RevertShaderChangeSail2 (Variables|Default|GetSails_Stage2))))
                (:then_1
                  (if (> (Variables|Default|GetThurster3Alpha) 0.0)
                    (CallFunction|RevertShaderChangeSail3 (Variables|Default|GetSails_Stage3))))))))
        (:then_1
          (goto _label Reset))
        (:then_2
          (goto _label_4 Reset))
        (:then_3
          (goto _label_3 Reset))))
    (:NewEnumerator2
      (Utilities|FlowControl|Sequence
        (:then_0
          (Utilities|FlowControl|DoOnce false :!label _label_3
            (:Completed
              (CallFunction|ChangeShaderParamSail2 (Variables|Default|GetSails_Stage2) "Opacity")
              (CallFunction|ChangeShaderParam (Variables|Default|GetSails_Stage1) "Opacity"))))
        (:then_1
          (goto _label_4 Reset))
        (:then_2
          (goto _label Reset))
        (:then_3
          (goto _label_2 Reset))))
    (:NewEnumerator3
      (Utilities|FlowControl|Sequence
        (:then_0
          (Utilities|FlowControl|DoOnce false :!label _label_4
            (:Completed
              (CallFunction|ChangeShaderParamSail3 (Variables|Default|GetSails_Stage3) "Opacity")
              (CallFunction|ChangeShaderParam (Variables|Default|GetSails_Stage1) "Opacity")
              (CallFunction|ChangeShaderParamSail2 (Variables|Default|GetSails_Stage2) "Opacity"))))
        (:then_1
          (goto _label_3 Reset))
        (:then_2
          (goto _label Reset))
        (:then_3
          (goto _label_2 Reset))))))

(event Custom|ChangeShaderParam
  (params (ObjectWithMat :type Mesh%20Component%20Object%20Reference) (ParameterName :type Name))
  ;[0.1198 0.2804 0.5052] Sail Timelines for transition
  (bind _alpha (Timeline|ChangeShaderTimeline Play)
    (:Update
      (Rendering|Material|SetScalarParameterValueonMaterials ObjectWithMat ParameterName _alpha))))

(event Custom|RevertShaderChange
  (params (ObjectWithMat :type Mesh%20Component%20Object%20Reference))
  ;[0.1198 0.2804 0.5052] Sail Timelines for transition
  (bind _alpha (Timeline|ChangeShaderTimeline Reverse)
    (:Update
      (Rendering|Material|SetScalarParameterValueonMaterials (stale Custom|ChangeShaderParam ObjectWithMat) (stale Custom|ChangeShaderParam ParameterName) _alpha))))

(event Custom|ChangeShaderParamSail2
  (params (ObjectWithMat :type Mesh%20Component%20Object%20Reference) (ParameterName :type Name))
  ;[0.1198 0.2804 0.5052] Sail Timelines for transition
  (bind _alpha (Timeline|ChangeShaderTimelineSail2 Play)
    (:Update
      (Rendering|Material|SetScalarParameterValueonMaterials ObjectWithMat ParameterName _alpha)
      (Variables|Default|SetThurster2Alpha _alpha))))

(event Custom|RevertShaderChangeSail2
  (params (ObjectWithMat :type Mesh%20Component%20Object%20Reference))
  ;[0.1198 0.2804 0.5052] Sail Timelines for transition
  (bind _alpha (Timeline|ChangeShaderTimelineSail2 Reverse)
    (:Update
      (Rendering|Material|SetScalarParameterValueonMaterials (stale Custom|ChangeShaderParamSail2 ObjectWithMat) (stale Custom|ChangeShaderParamSail2 ParameterName) _alpha)
      (Variables|Default|SetThurster2Alpha _alpha))))

(event EventBeginPlay
  ;[0 0 0] Get reference to the boat
  (bind _asboat (Utilities|Casting|CastToboat (Actor|GetParentActor)))
  (Variables|Default|SetAs%20Boat _asboat)
  ;[0 0 0] Makes an event which gets called as often as we allocate also avoiding event tick
  (Utilities|Time|SetTimerbyEvent (EventDispatchers|CreateEvent :!event Custom|ChangeSails) 0.1 true)
  (Utilities|Time|SetTimerbyEvent (EventDispatchers|CreateEvent :!event Custom|ChangeSailShaderCallable) 0.1 true))

(fn ConstructionScript)