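; Destructible wood, copper or metal asteroid that travels along a spline path via a timeline, with a Niagara system matching its material.
; First damage adds a material-specific Chaos geometry collection.
; A break event or depleted health triggers sparks and camera shake, stops movement, spawns a resource drop and notifies the GameState.
; A timeline then shrinks the dissolve radius in a material parameter collection before destroying the actor.
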(event Custom|MoveOnPath
  (bind _pathref (Variables|Default|GetpathRef))
  (bind _track (Variables|/Game/VFX/VFX/BIS/Path.Path_C|GetTrack _pathref))
  (if (not (Variables|Default|GetbeingDestroyed?))
    (Components|Timeline|SetPlayRate (Variables|Default|GetPathMoverTimeline) (Math|Float|%(Float) (+ (Variables|Default|GetDuration) (Math|Random|RandomFloatinRange 0.0008 0.003)) (Spline|GetSplineLength (Variables|/Game/VFX/VFX/BIS/Path.Path_C|GetTrack (Variables|Default|GetpathRef)))))
    (Utilities|FlowControl|Sequence
      (:then_0
        (bind _alpha (Timeline|PathMoverTimeline Play)
          (:Update
            (Variables|Default|SetAlpha _alpha)
            (if (Utilities|IsValid _track)
              (Transformation|SetActorLocationAndRotation (Spline|GetLocationatDistanceAlongSpline _track (Math|Float|Lerp 0.0 (Spline|GetSplineLength (Variables|/Game/VFX/VFX/BIS/Path.Path_C|GetTrack (Variables|Default|GetpathRef))) (Variables|Default|GetAlpha)) "World") (Spline|GetRotationatDistanceAlongSpline (Variables|/Game/VFX/VFX/BIS/Path.Path_C|GetTrack (Variables|Default|GetpathRef)) (Math|Float|Lerp 0.0 (Spline|GetSplineLength (Variables|/Game/VFX/VFX/BIS/Path.Path_C|GetTrack (Variables|Default|GetpathRef))) (Variables|Default|GetAlpha)) "World") true)
              (Class|PawnMovementComponent|AddInputVector (Variables|Default|GetFloatingPawnMovement) (Math|Vector|GetForwardVector (Variables|Default|GetParentHolder)) false)))))
      (:then_1
        (Timeline|PathMoverTimeline SetNewTime)))))

(event Custom|Killed
  (CallFunction|StopTimeline)
  (CallFunction|SpawnCrate (Variables|Default|GetE%20Type%20Of%20Mat))
  (Class|INTGameplayEvents|AsteroidDestroyed(Message) (Game|GetGameState) (Variables|Default|GetpathRef) (Variables|Default|GetE%20Type%20Of%20Mat)))

(event Custom|RemoveBoatStaticParts
  (params (MeshArray :type Array%20of%20Static%20Mesh%20Component%20Object%20References))
  ;[1 1 1] Destruction System
  (for (_array_element _array_index) MeshArray
    (if (Utilities|Array|IsValidIndex MeshArray _array_index)
      (Components|DestroyComponent _array_element)))
  (Utilities|Array|Clear MeshArray))

(event Custom|RefreshNiagaraSys
  (bind _niagara (Variables|Default|GetNiagara))
  (switch Utilities|FlowControl|Switch|SwitchonTypesOfResources (Variables|Default|GetE%20Type%20Of%20Mat)
    (:NewEnumerator0
      (Class|NiagaraComponent|SetAsset _niagara "/Game/VFX/VFX/BIS/Asteroid_Wood.Asteroid_Wood" true))
    (:NewEnumerator1
      (Class|NiagaraComponent|SetAsset _niagara "/Game/VFX/VFX/BIS/Asteroid_Copper.Asteroid_Copper" true))
    (:NewEnumerator2
      (Class|NiagaraComponent|SetAsset _niagara "/Game/VFX/VFX/BIS/Asteroid_Metal.Asteroid_Metal" true))))

(event Custom|OnChaosBreakEvent_Event
  (params (BreakEvent :type Chaos%20Break%20Event%20Structure%20%28by%20ref%29))
  (bind _returnvalue (Transformation|GetActorLocation))
  ;[1 1 1] Destruction System
  ;[1 1 1] Damage Handler
  (Utilities|FlowControl|DoOnce false
    (:Completed
      (Effects|SpawnEmitteratLocation "/Game/EpicContent/StarterContent/Particles/P_ShotSparkBack.P_ShotSparkBack" _returnvalue "0, 0, 0" "100.000000,100.000000,100.000000" true "AutoRelease")
      (Camera|PlayWorldCameraShake "/Game/KillingShake.KillingShake_C" _returnvalue 0.0 4.5e+04)
      (CallFunction|Killed)
      (CallFunction|FadeGeoCollection))))

(event Custom|SpawnCrate
  (params (eTypeOfMat :type TypesOfResources%20Enum :default "NewEnumerator0"))
  ;[1 1 1] Death Handler
  (bind _returnvalue (Game|SpawnActorfromClass "/Game/Core/Resources/ResourceDropAsteroid.ResourceDropAsteroid_C" (Math|Transform|MakeTransform (+ (Transformation|GetActorLocation) (Math|Vector|MakeVector (Math|Random|RandomFloatinRange -2e+03 6e+03) (Math|Random|RandomFloatinRange -2e+03 4e+03) (Math|Random|RandomFloatinRange -1e+03 1e+03))) (Math|Random|RandomRotator true) "1.000000,1.000000,1.000000") "AdjustIfPossibleButAlwaysSpawn" 0 0))
  (Variables|/Game/Core/Resources/ResourceDropAsteroid.ResourceDropAsteroid_C|SeteTypeOfMat _returnvalue eTypeOfMat))

(event Custom|FadeGeoCollection
  ;[1 1 1] Destruction System
  (bind _fade_time (Timeline|FadeGeoTimeline Play)
    (:Update
      (Rendering|Material|SetScalarParameterValue "/Game/VFX/Dissolve/DissolveMatCollection.DissolveMatCollection" "Radius" (Math|Float|Lerp 9e+04 0.0 _fade_time) :!class /Script/Engine.KismetMaterialLibrary))
    (:Finished
      (Actor|DestroyActor))))

(event Custom|CheckHealth
  ;[1 1 1] Destruction System
  (if (!= (Variables|Default|Gethealth) (Variables|Default|GetmaxHealth))
    (Variables|Default|SetbeingDestroyed? true)
    (Utilities|FlowControl|DoOnce false
      (:Completed
        (CallFunction|SwapModelwithGeoCache)))))

(event Custom|SwapModelWithGeoCache
  ;[1 1 1] Destruction System
  (bind _returnvalue (CallFunction|RefreshGeometryCollectionFunc))
  (EventDispatchers|AssignOnChaosBreakEvent _returnvalue (delegate Custom|OnChaosBreakEvent_Event))
  (Rendering|Material|SetScalarParameterValue "/Game/VFX/Dissolve/DissolveMatCollection.DissolveMatCollection" "Radius" 9e+04 :!class /Script/Engine.KismetMaterialLibrary))

(event Custom|StopTimeline
  (bind _pathref (Variables|Default|GetpathRef))
  (bind _track (Variables|/Game/VFX/VFX/BIS/Path.Path_C|GetTrack _pathref))
  (bind _alpha (Timeline|PathMoverTimeline Stop)
    (:Update
      (Variables|Default|SetAlpha _alpha)
      (if (Utilities|IsValid _track)
        (Transformation|SetActorLocationAndRotation (Spline|GetLocationatDistanceAlongSpline _track (Math|Float|Lerp 0.0 (Spline|GetSplineLength (Variables|/Game/VFX/VFX/BIS/Path.Path_C|GetTrack (Variables|Default|GetpathRef))) (Variables|Default|GetAlpha)) "World") (Spline|GetRotationatDistanceAlongSpline (Variables|/Game/VFX/VFX/BIS/Path.Path_C|GetTrack (Variables|Default|GetpathRef)) (Math|Float|Lerp 0.0 (Spline|GetSplineLength (Variables|/Game/VFX/VFX/BIS/Path.Path_C|GetTrack (Variables|Default|GetpathRef))) (Variables|Default|GetAlpha)) "World") true)
        (Class|PawnMovementComponent|AddInputVector (Variables|Default|GetFloatingPawnMovement) (Math|Vector|GetForwardVector (Variables|Default|GetParentHolder)) false)))))

(event EventBeginPlay
  (if (Variables|Default|GetActivePath) :!label _label
    (if (and (Utilities|IsValid (Variables|Default|GetPathMoverTimeline)) (Utilities|IsValid (Variables|Default|GetpathRef)))
      (CallFunction|RefreshNiagaraSys)
      (CallFunction|MoveonPath)
      (else
        (Utilities|FlowControl|RetriggerableDelay 0.2)
        (goto _label)))))

(event Game|Damage|EventAnyDamage
  (params (Damage :type Float%20%28single-precision%29) (DamageType :type Damage%20Type%20Object%20Reference) (InstigatedBy :type Controller%20Object%20Reference) (DamageCauser :type Actor%20Object%20Reference))
  (bind _returnvalue (Transformation|GetActorLocation))
  ;[1 1 1] Damage Handler
  (Utilities|FlowControl|Sequence
    (:then_0
      (Variables|Default|Sethealth (- (Variables|Default|Gethealth) Damage))
      (CallFunction|CheckHealth))
    (:then_1
      (if (not (> (Variables|Default|Gethealth) 0.0))
        (Utilities|FlowControl|DoOnce false
          (:Completed
            (Effects|SpawnEmitteratLocation "/Game/EpicContent/StarterContent/Particles/P_ShotSparkBack.P_ShotSparkBack" _returnvalue "0, 0, 0" "100.000000,100.000000,100.000000" true "AutoRelease")
            (Camera|PlayWorldCameraShake "/Game/KillingShake.KillingShake_C" _returnvalue 0.0 4.5e+04)
            (CallFunction|Killed)
            (CallFunction|FadeGeoCollection)))))))

(fn ConstructionScript)

(fn RefreshGeometryCollectionFunc
  (switch Utilities|FlowControl|Switch|SwitchonTypesOfResources (Variables|Default|GetE%20Type%20Of%20Mat)
    (:NewEnumerator0
      (bind _returnvalue (AddComponent|AddGeometryCollectionComponent false))
      (return _returnvalue))
    (:NewEnumerator1
      (bind _returnvalue_2 (AddComponent|AddGeometryCollectionComponent false))
      (return _returnvalue_2))
    (:NewEnumerator2
      (bind _returnvalue_3 (AddComponent|AddGeometryCollectionComponent false))
      (return _returnvalue_3))))