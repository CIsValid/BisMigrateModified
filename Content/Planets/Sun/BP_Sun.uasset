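; BP_Sun is the Sun actor in the planets content, carrying main, left and right solar bases, each with outer and inner parts.
; On BeginPlay it binds six RotatingMovement components to those parts, so each spins independently of the actor's root.
; SetUpdatedComponent redirects each movement to its own part, and the graph's comments group them by base size and axis.
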(event EventBeginPlay
  ;[1 1 1] Big base
  (Components|Movement|SetUpdatedComponent (Variables|Default|GetRotatingMovementHugeBase) (Variables|Default|GetSolarBase_Main_Outer))
  (Components|Movement|SetUpdatedComponent (Variables|Default|GetRotatingMovementSmallBase) (Variables|Default|GetSolarBase_Left_Outer))
  (Components|Movement|SetUpdatedComponent (Variables|Default|GetRotatingMovementHugeBase1) (Variables|Default|GetSolarBase_Right_Outer))
  ;[1 1 1] Small
  (Components|Movement|SetUpdatedComponent (Variables|Default|GetRotatingMovementHugeBase2) (Variables|Default|GetSolarBase_Main_Inner))
  (Components|Movement|SetUpdatedComponent (Variables|Default|GetRotatingMovementHugeBase3) (Variables|Default|GetSolarBase_Right_Inner))
  (Components|Movement|SetUpdatedComponent (Variables|Default|GetRotatingMovementHugeBase4) (Variables|Default|GetSolarBase_Left_Inner)))

(fn ConstructionScript)